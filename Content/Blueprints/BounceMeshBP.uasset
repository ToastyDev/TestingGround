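; BounceMeshBP is an actor whose cube reacts to FirstPersonProjectile hits by driving an impact effect in its material.
; On BeginPlay it creates a dynamic material instance on the cube.
; Each projectile hit writes the impact point to the "pos" parameter, prints the normal and restarts the Bounce timeline.
; The timeline scales the hit normal into the "impact" vector, leaving the visual response to the material.
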(event `self.ReceiveBeginPlay`
  (bind _returnvalue (`PrimitiveComponent.CreateDynamicMaterialInstance` (`self.Cube`) 0 null "None"))
  (set `self.Material` _returnvalue))

(event `self.Cube.OnComponentHit`
  (params (HitComponent :type "PrimitiveComponent Object Reference") (OtherActor :type "Actor Object Reference") (OtherComp :type "PrimitiveComponent Object Reference") (NormalImpulse :type "Vector Structure") (Hit :type "HitResult Structure (by ref)"))
  (bind _material (`self.Material`))
  (cast `/Game/FirstPersonBP/Blueprints/FirstPersonProjectile` OtherActor)
  (`MaterialInstanceDynamic.SetVectorParameterValue` _material "pos" (`KismetMathLibrary.Conv_VectorToLinearColor` Hit_ImpactPoint))
  (`KismetSystemLibrary.PrintString` (`KismetStringLibrary.Conv_VectorToString` Hit_Normal))
  (bind (_direction _newtrack_0) (`Timeline|Bounce` :!via `PlayFromStart`)
    (:`Update`
      (`MaterialInstanceDynamic.SetVectorParameterValue` _material "impact" (`KismetMathLibrary.Conv_VectorToLinearColor` (* Hit_Normal (* _newtrack_0 50.0)))))))

(fn `UserConstructionScript`)